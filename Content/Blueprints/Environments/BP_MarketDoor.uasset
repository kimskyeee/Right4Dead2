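; Market double door that swings open and closed on interaction and sets off an alarm the first time it opens.
; InteractionDoor toggles the open state, playing or reversing a Timeline that rotates the left and right hinges.
; The first opening spawns an attenuated alarm sound at AlarmLocation and starts horde music through BP_SoundManager, found on BeginPlay.
; StopAlarm silences the alarm, clears the Alarming flag and disables actor tick.
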(event `self.ReceiveBeginPlay`
  (bind _returnvalue (`GameplayStatics.GetActorOfClass` "/Game/Blueprints/BP_SoundManager.BP_SoundManager_C"))
  (set `self.SoundManager` _returnvalue))

(event `self.InteractionDoor`
  (bind _alarmlocation (`self.AlarmLocation`))
  (bind _output_get (set `self.bIsOpen` (not (`self.bIsOpen`))))
  (if _output_get
    (`|ExecutionSequence`
      (:`then_0`
        (if (`self.bFirst`)
          (set `self.bFirst` false)
          (bind _returnvalue (`GameplayStatics.SpawnSoundAtLocation` (`self.AlarmSound`) (`SceneComponent.K2_GetComponentLocation` _alarmlocation) (`SceneComponent.K2_GetComponentRotation` _alarmlocation) 1.0 1.0 0.0 "/Game/Assets/Sounds/MarketDoorAlarm/SA_MarketDoorAlarm.SA_MarketDoorAlarm" null))
          (set `self.AlarmComponent` _returnvalue)
          (set `self.bAlarming` true)
          (`/Game/Blueprints/BP_SoundManager.StartHordeBGM` (`self.SoundManager`))))
      (:`then_1`
        (bind (_direction _righthingerottrack _lefthingerottrack) (`Timeline|Timeline` :!label _label)
          (:`Update`
            (`SceneComponent.K2_SetRelativeRotation` (`self.RightHinge`) (`KismetMathLibrary.MakeRotator` 0.0 0.0 _righthingerottrack) false false)
            (`SceneComponent.K2_SetRelativeRotation` (`self.LeftHinge`) (`KismetMathLibrary.MakeRotator` 0.0 0.0 _lefthingerottrack) false false)))))
    (else
      (goto _label :!via `Reverse`))))

(event `self.StopAlarm`
  (bind _alarmcomponent (`self.AlarmComponent`))
  (`/Engine/EditorBlueprintResources/StandardMacros.IsValid` _alarmcomponent
    (:`Is Valid`
      (`AudioComponent.Stop` _alarmcomponent)
      (set `self.bAlarming` false)
      (`self.SetActorTickEnabled` false))))

(fn `UserConstructionScript`)