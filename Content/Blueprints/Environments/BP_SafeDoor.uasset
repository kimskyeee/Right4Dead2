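; BP_SafeDoor is an interactable safe door that swings open and closed on its hinge.
; Each InteractionDoor call toggles IsOpen and plays or reverses a Timeline that drives the Hinge's relative yaw.
; A First flag makes the initial close reverse from the timeline's end.
; When the timeline finishes with the door closed, it calls OnDoorClosed on the BP_ClearTriggerBox found at BeginPlay.
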(event `self.ReceiveBeginPlay`
  (bind _returnvalue (`GameplayStatics.GetActorOfClass` "/Game/Blueprints/Survivor/Item/BP_ClearTriggerBox.BP_ClearTriggerBox_C"))
  (set `self.ClearTriggerBox` _returnvalue))

(event `self.InteractionDoor`
  (bind _output_get (set `self.bIsOpen` (not (`self.bIsOpen`))))
  (if _output_get
    (bind (_direction _rottrack) (`Timeline|Timeline` :!label _label)
      (:`Update`
        (`SceneComponent.K2_SetRelativeRotation` (`self.Hinge`) (`KismetMathLibrary.MakeRotator` 0.0 0.0 _rottrack) false false))
      (:`Finished`
        (if (not (`self.bIsOpen`))
          (`/Game/Blueprints/Survivor/Item/BP_ClearTriggerBox.OnDoorClosed` (`self.ClearTriggerBox`)))))
    (elif (`self.bFirst`)
      (set `self.bFirst` false)
      (goto _label :!via `ReverseFromEnd`)
      (else
        (goto _label :!via `Reverse`)))))

(fn `UserConstructionScript`)