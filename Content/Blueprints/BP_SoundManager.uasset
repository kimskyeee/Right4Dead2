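; BP_SoundManager is a sound manager actor that switches background music between peace and horde tracks.
; It holds two audio components, PeaceMusicCue and HordeMusicCue, and stops the horde track on BeginPlay.
; Custom events StartPeaceBGM and StartHordeBGM stop the opposite track and play their own from the start, while StopAll silences both.
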(event `self.ReceiveBeginPlay`
  (`AudioComponent.Stop` (`self.HordeMusicCue`)))

(event `StartPeaceBGM`
  (`AudioComponent.Stop` (`self.HordeMusicCue`))
  (`AudioComponent.Play` (`self.PeaceMusicCue`) 0.0))

(event `StartHordeBGM`
  (`AudioComponent.Stop` (`self.PeaceMusicCue`))
  (`AudioComponent.Play` (`self.HordeMusicCue`) 0.0))

(event `StopAll`
  (`AudioComponent.Stop` (`self.HordeMusicCue`))
  (`AudioComponent.Stop` (`self.PeaceMusicCue`)))

(fn `UserConstructionScript`)