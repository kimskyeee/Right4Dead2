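; Audio component for the common zombie that plays its chase, footstep, attack, hit and death sounds.
; On begin play it spawns looping-controlled chase and footstep sounds attached to the owner's root, stopped until needed.
; Entering Chase starts both; entering Dead stops them and plays a death cue.
; Punch, bullet hit, shove and dismemberment events each play a one-shot cue at the owner's location.
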(event `self.ReceiveBeginPlay`
  (bind _returnvalue (`GameplayStatics.SpawnSoundAttached` (`self.ChaseSoundCue`) (`Actor.RootComponent` (`self.GetOwner`)) "None" (0.0 0.0 0.0) (struct) "KeepRelativeOffset" true 1.0 1.0 0.0 "/Game/Assets/Sounds/Zombie/ZombieSoundAttenuation.ZombieSoundAttenuation" null false))
  (bind _output_get (set `self.ChaseAudioComponent` _returnvalue))
  (`AudioComponent.Stop` _output_get)
  (bind _returnvalue_2 (`GameplayStatics.SpawnSoundAttached` (`self.FootstepSoundCue`) (`Actor.RootComponent` (`self.GetOwner`)) "None" (0.0 0.0 0.0) (struct) "KeepRelativeOffset" true 0.5 1.0 0.0 "/Game/Assets/Sounds/Zombie/ZombieSoundAttenuation.ZombieSoundAttenuation" null false))
  (bind _output_get_2 (set `self.FootstepAudioComponent` _returnvalue_2))
  (`AudioComponent.Stop` _output_get_2))

(event `self.OnChangedState`
  (params (BeforeState :type "EZombieState Enum (by ref)" :default "EZS_Idle") (AfterState :type "EZombieState Enum (by ref)" :default "EZS_Idle"))
  (switch `EZombieState` AfterState
    (:`EZS_Chase`
      (`AudioComponent.Play` (`self.ChaseAudioComponent`) 0.0)
      (`AudioComponent.Play` (`self.FootstepAudioComponent`) 0.0))
    (:`EZS_Dead`
      (`AudioComponent.Stop` (`self.ChaseAudioComponent`))
      (`AudioComponent.Stop` (`self.FootstepAudioComponent`))
      (`GameplayStatics.PlaySoundAtLocation` (`self.DieSoundCue`) (`Actor.K2_GetActorLocation` (`self.Owner`)) (struct) 1.0 1.0 0.0 "/Game/Assets/Sounds/Zombie/ZombieSoundAttenuation.ZombieSoundAttenuation" null null null))))

(event `self.OnNormalAttacked`
  (`GameplayStatics.PlaySoundAtLocation` (`self.PunchSoundCue`) (`Actor.K2_GetActorLocation` (`self.Owner`)) (struct) 1.0 1.0 0.0 "/Game/Assets/Sounds/Zombie/ZombieSoundAttenuation.ZombieSoundAttenuation" null null null))

(event `self.OnBulletHit`
  (params (HitInfo :type "HitResult Structure (by ref)"))
  (`GameplayStatics.PlaySoundAtLocation` (`self.HitByBulletSoundCue`) (`Actor.K2_GetActorLocation` (`self.Owner`)) (struct) 0.4 1.0 0.0 "/Game/Assets/Sounds/Zombie/ZombieSoundAttenuation.ZombieSoundAttenuation" null null null))

(event `self.OnDismemberment`
  (`GameplayStatics.PlaySoundAtLocation` (`self.DismembermentSoundCue`) (`Actor.K2_GetActorLocation` (`self.Owner`)) (struct) 1.0 1.0 0.0 "/Game/Assets/Sounds/Zombie/ZombieSoundAttenuation.ZombieSoundAttenuation" null null null))

(event `self.OnShove`
  (`GameplayStatics.PlaySoundAtLocation` (`self.HitShoveSoundCue`) (`Actor.K2_GetActorLocation` (`self.Owner`)) (struct) 1.0 1.0 0.0 "/Game/Assets/Sounds/Zombie/ZombieSoundAttenuation.ZombieSoundAttenuation" null null null))