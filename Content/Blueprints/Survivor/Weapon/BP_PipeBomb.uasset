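; BP_PipeBomb is the survivor's pipe bomb weapon Blueprint, handling its accelerating warning beep.
; The PlayBeepSound event accumulates the delta time passed in and plays a 2D beep whenever the total exceeds the current interval.
; Each beep resets the timer and lerps the interval toward a short minimum, so the beeps speed up with diminishing steps.
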(event `self.PlayBeepSound`
  (params (DeltaTime :type "Float (single-precision)"))
  ; 시간을 더해줘라
  (set `self.CurrentBeepTime` (+ DeltaTime (`self.CurrentBeepTime`)))
  ; 삐삐거릴 시간이 되었으니 삐삐거려라
  (if (> (`self.CurrentBeepTime`) (`self.BeepInterval`))
    (set `self.CurrentBeepTime` 0.0)
    (`GameplayStatics.PlaySound2D` "/Game/Assets/Sounds/WeaponNAttack/PipeBomb/pipebomb_beep.pipebomb_beep" 1.0 1.0 0.0 null null)
    ; 다음엔 더 빨리 삐삐거리게 하자
    (set `self.BeepInterval` (`KismetMathLibrary.Lerp` (`self.BeepInterval`) 0.08 0.2))))

(fn `UserConstructionScript`
  (`parent.UserConstructionScript`))