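; BP_CokeDelivery is an interactable survivor-item Blueprint for a Coke delivery point with a hinged door, flagged as a Coke delivery on BeginPlay.
; Each InteractionDelivery call toggles IsOpen, and a Timeline plays to swing the Hinge open along roll only if IsCanOpen is also true, otherwise it reverses.
; IsCanOpen is set outside this graph and, per the comments, means the held weapon is a Coke bottle.
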(event `self.ReceiveBeginPlay`
  (set `self.bIsOpen` false)
  (set `self.bIsCokeDelivery` true))

(event `self.InteractionDelivery`
  ; 문이 열리고 있는중인지
  (bind _output_get (set `self.bIsOpen` (not (`self.bIsOpen`))))
  (if (and _output_get (`self.bIsCanOpen`))
    (bind (_direction _rottrack) (`Timeline|Timeline` :!label _label)
      (:`Update`
        (`SceneComponent.K2_SetRelativeRotation` (`self.Hinge`) (`KismetMathLibrary.MakeRotator` (* _rottrack -1.0)) false false)))
    (else
      (goto _label :!via `Reverse`))))

(fn `UserConstructionScript`)