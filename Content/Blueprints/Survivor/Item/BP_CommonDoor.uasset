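; BP_CommonDoor is a Survivor item Blueprint for a hinged door that swings open and closed on interaction.
; InteractionCommonDoor toggles IsOpen, then plays a Timeline that sets the Hinge yaw when IsOpen and IsCanOpen are both true, otherwise reverses it.
; IsCanOpen starts false and is never set true here, and IsOpen still flips when the door cannot open.
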(event `self.ReceiveBeginPlay`
  (set `self.bIsCanOpen` false)
  (set `self.bIsOpen` false))

(event `self.InteractionCommonDoor`
  (bind _output_get (set `self.bIsOpen` (not (`self.bIsOpen`))))
  (if (and _output_get (`self.bIsCanOpen`))
    (bind (_direction _rottrack) (`Timeline|Timeline` :!label _label)
      (:`Update`
        (`SceneComponent.K2_SetRelativeRotation` (`self.Hinge`) (`KismetMathLibrary.MakeRotator` 0.0 0.0 _rottrack) false false)))
    (else
      (goto _label :!via `Reverse`))))

(fn `UserConstructionScript`)