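; BP_ClearTriggerBox is a survivor-side trigger volume that loads the game clear map when the safe door closes with a survivor inside.
; At BeginPlay it caches a reference to the level's BP_SafeDoor, and overlap events toggle a single OverlapSurvivor flag rather than counting survivors.
; Its OnDoorClosed event checks that flag and, if set, opens GameClearMap; this graph neither binds nor calls that event.
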(event `self.ReceiveBeginPlay`
  (bind _returnvalue (`GameplayStatics.GetActorOfClass` "/Game/Assets/Environments/SafeDoor/BP_SafeDoor.BP_SafeDoor_C"))
  (`/Engine/EditorBlueprintResources/StandardMacros.IsValid` _returnvalue
    (:`Is Valid`
      (set `self.SafeDoor` _returnvalue))))

(event `self.ReceiveActorBeginOverlap`
  (params (OtherActor :type "Actor Object Reference"))
  (cast `/Game/Blueprints/Survivor/BP_SurvivorCharacter` OtherActor)
  (set `self.bOverlapSurvivor` true))

(event `self.ReceiveActorEndOverlap`
  (params (OtherActor :type "Actor Object Reference"))
  (cast `/Game/Blueprints/Survivor/BP_SurvivorCharacter` OtherActor)
  (set `self.bOverlapSurvivor` false))

(event `OnDoorClosed`
  (if (`self.bOverlapSurvivor`)
    (`GameplayStatics.OpenLevelBySoftObjectPtr` "/Game/Maps/GameClearMap.GameClearMap")))

(fn `UserConstructionScript`)