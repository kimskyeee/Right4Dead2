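; Survivor character Blueprint holding unfinished, disconnected prototypes for crosshair UI and a trace-based "Crow" attack; none of its events run any logic.
; Crow and EndCrow are empty stubs, with notes on line tracing during a montage between animation notifies.
; Unwired fragments start and clear a repeating-trace timer handle, apply damage to line trace hits, and map velocity to crosshair spread.
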(event `self.ReceiveTick`
  (params (DeltaSeconds :type "Float (single-precision)")))

(event `self.ReceiveBeginPlay`)

(event `Crow`
  ; 몽타주 재생하는 동안에 라인트레이스 하는법
)

(event `EndCrow`
  ; 몽타주 재생하는 동안에 라인트레이스 하는법
  ;; 이것도
)

(fn `UserConstructionScript`)